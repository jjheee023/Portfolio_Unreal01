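; Spline movement Blueprint that carries a referenced actor along a spline in a continuous loop.
; A timeline, with play rate set from a length variable on BeginPlay, lerps distance up to the last spline point to set world location, restarting when finished.
; Rotation always follows the local-space tangent at distance zero, so it ignores progress along the path.
; The construction script places the actor at the first point's local-space location.
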(event `Play timeline`
  (bind _spline (`self.Spline`))
  (bind _spline_2 (`self.Spline`))
  (bind _actor (`self.actor`))
  (bind (_direction _newtrack_0) (`Timeline|Timeline_0` :!via `PlayFromStart`)
    (:`Update`
      (`self.K2_SetActorLocation` _actor (`SplineComponent.GetLocationAtDistanceAlongSpline` _spline_2 (`KismetMathLibrary.Lerp` 0.0 (`SplineComponent.GetDistanceAlongSplineAtSplinePoint` _spline (- (`SplineComponent.GetNumberOfSplinePoints` _spline) 1)) _newtrack_0) "World") false false)
      (`self.K2_SetActorRotation` _actor (`KismetMathLibrary.Conv_VectorToRotator` (`SplineComponent.GetTangentAtDistanceAlongSpline` _spline_2 0.0 "Local")) false))
    (:`Finished`
      (`self.Play timeline`))))

(event `self.ReceiveBeginPlay`
  (`TimelineComponent.SetPlayRate` (`self.Timeline_0`) (/ 1.0 (`self.Timeline lenth`)))
  (`self.Play timeline`))

(fn `UserConstructionScript`
  (`self.K2_SetActorLocation` (`self.actor`) (`SplineComponent.GetLocationAtSplinePoint` (`self.Spline`) 0 "Local") false false))